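; BP_PersoATuer is a killable target character that reports an objective to the player when it dies.
; AnyDamage subtracts from Health, playing a sword-and-shield impact montage while it survives.
; At zero or below it plays a death montage, waits briefly, calls OnObjectivesIDCalled on BP_PersoPrincipal with its ObjectiveID, then destroys itself.
; If the player character cast fails, the actor is not destroyed.
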(event `self.ReceiveAnyDamage`
  (params (Damage :type "Float (single-precision)") (DamageType :type "DamageType Object Reference") (InstigatedBy :type "Controller Object Reference") (DamageCauser :type "Actor Object Reference"))
  (bind _output_get (set `self.health` (- (`self.health`) Damage)))
  (if (<= _output_get 0.0)
    (`self.PlayAnimMontage` "/Game/Character/Animation/Sword_And_Shield_Death_Montage.Sword_And_Shield_Death_Montage")
    (`KismetSystemLibrary.Delay` 3.5)
    (bind _asbp_perso_principal (cast `/Game/Character/BP_PersoPrincipal` (`GameplayStatics.GetPlayerCharacter` 0)))
    (`/Game/Character/BP_PersoPrincipal.OnObjectivesIDCalled` _asbp_perso_principal (`self.ObjectiveID`))
    (`self.K2_DestroyActor`)
    (else
      (bind _returnvalue (`self.PlayAnimMontage` "/Game/Character/Animation/Sword_And_Shield_Impact_Montage.Sword_And_Shield_Impact_Montage"))
      (`KismetSystemLibrary.Delay` _returnvalue))))

(fn `UserConstructionScript`)