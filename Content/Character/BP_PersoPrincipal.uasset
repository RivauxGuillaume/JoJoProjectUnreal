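; BP_PersoPrincipal is the main player character, handling movement, mouse look and interaction with objects.
; Movement follows control yaw, while mouse axes drive controller yaw and pitch.
; Every tick, a short line trace along the actor's forward vector stores any hit actor implementing the interaction interface and sends it a look-at message.
; Pressing Interact messages that actor and broadcasts its returned value through the OnObjectivesIDCalled dispatcher.
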(event `InputAxis|Tourner`
  (params (AxisValue :type "Float (single-precision)"))
  ;[1 1 1] Mouvement De Souris
  (`self.AddControllerYawInput` AxisValue))

(event `InputAxis|SedeplacerAvant/Arriere`
  (params (AxisValue :type "Float (single-precision)"))
  (bind _returnvalue (`GameplayStatics.GetPlayerCharacter` 0))
  ;[1 1 1] Se Déplacer
  (`self.AddMovementInput` _returnvalue (`KismetMathLibrary.GetForwardVector` (`KismetMathLibrary.MakeRotator` 0.0 0.0 (.yaw (`self.GetControlRotation` _returnvalue)))) AxisValue false))

(event `InputAxis|RegarderEnHaut/Bas`
  (params (AxisValue :type "Float (single-precision)"))
  ;[1 1 1] Mouvement De Souris
  (`self.AddControllerPitchInput` AxisValue))

(event `InputAxis|AllerAGauche/Droite`
  (params (AxisValue :type "Float (single-precision)"))
  (bind _returnvalue (`GameplayStatics.GetPlayerCharacter` 0))
  ;[1 1 1] Se Déplacer
  (`self.AddMovementInput` _returnvalue (`KismetMathLibrary.GetRightVector` (`KismetMathLibrary.MakeRotator` 0.0 0.0 (.yaw (`self.GetControlRotation` _returnvalue)))) AxisValue false))

(event `self.ReceiveTick`
  (params (DeltaSeconds :type "Float (single-precision)"))
  (`self.InteractTrace`))

(event `InputAction|Interact`
  (params (Key :type "Key Structure"))
  (:`Pressed`
    (bind _lookatactor (`self.LookAtActor`)
      (:`then`
        (bind _objectiveid (message `/Game/IInteractionIntecface.InteractWith` _lookatactor))
        (`self.OnObjectivesIDCalled` _objectiveid))
      (:`else`))))

(fn `InteractTrace`
  (bind _returnvalue (`GameplayStatics.GetPlayerCharacter` 0))
  (bind _returnvalue_2 (`self.K2_GetActorLocation` _returnvalue))
  (bind (_outhit _returnvalue_3) (`KismetSystemLibrary.LineTraceSingle` :`Start` _returnvalue_2 :`End` (+ _returnvalue_2 (* (`self.GetActorForwardVector` _returnvalue) 200.0)) :`TraceChannel` "TraceTypeQuery2" :`DrawTime` 2.0))
  (if _returnvalue_3
    (bind (_bblockinghit _binitialoverlap _time _distance _location _impactpoint _normal _impactnormal _physmat _hitactor) (`GameplayStatics.BreakHitResult` _outhit))
    (if (`KismetSystemLibrary.DoesImplementInterface` _hitactor "/Game/IInteractionIntecface.IInteractionIntecface_C")
      (bind _output_get (set `self.LookAtActor` _hitactor))
      (message `/Game/IInteractionIntecface.LookAt` _output_get)
      (else
        (set `self.LookAtActor` null)))
    (else
      (set `self.LookAtActor` null))))

(fn `UserConstructionScript`)